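; Breakable lamp actor that goes dark when a LowBall_BP or Whisky_BP actor overlaps it.
; Two duplicate overlap branches, one per class, wait briefly, hide the point and spot lights, and spawn a short-lived spark emitter at the point light.
; An IsWorking flag, set at BeginPlay, gates both branches and clears only after the sparks are destroyed, with nothing restoring the lamp afterwards.
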(event EventBeginPlay
  (Variables|Default|SetisWorking true))

(event Collision|EventActorBeginOverlap
  (params (OtherActor :type Actor%20Object%20Reference))
  (Utilities|FlowControl|Sequence
    (:then_0
      (if (Variables|Default|GetisWorking)
        (Utilities|Casting|CastToLowBall_BP OtherActor)
        (Utilities|FlowControl|Delay 0.1)
        (Rendering|SetVisibility (Variables|Default|GetPointLight) false false)
        (Rendering|SetVisibility (Variables|Default|GetSpotLight1) false false)
        (bind _returnvalue (Effects|SpawnEmitteratLocation "/Game/StarterContent/Particles/P_Sparks.P_Sparks" (Transformation|GetWorldLocation (Variables|Default|GetPointLight)) "180.000000, 0, 0"))
        (Utilities|FlowControl|Delay 0.4)
        (Components|DestroyComponent _returnvalue)
        (Variables|Default|SetisWorking false)))
    (:then_1
      (if (Variables|Default|GetisWorking)
        (Utilities|Casting|CastToWhisky_BP OtherActor)
        (Utilities|FlowControl|Delay 0.1)
        (Rendering|SetVisibility (Variables|Default|GetPointLight) false false)
        (Rendering|SetVisibility (Variables|Default|GetSpotLight1) false false)
        (bind _returnvalue_2 (Effects|SpawnEmitteratLocation "/Game/StarterContent/Particles/P_Sparks.P_Sparks" (Transformation|GetWorldLocation (Variables|Default|GetPointLight)) "180.000000, 0, 0"))
        (Utilities|FlowControl|Delay 0.4)
        (Components|DestroyComponent _returnvalue_2)
        (Variables|Default|SetisWorking false)))))

(event EventTick
  (params (DeltaSeconds :type Float%20%28single-precision%29)))

(fn ConstructionScript)