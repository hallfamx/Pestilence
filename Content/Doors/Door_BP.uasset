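; Door actor that the player can open and close or peek through with a blended camera view.
; FrontOpen overlap enables input and opens a Gate shared by Interact and Peek.
; Interact toggles the door through a FlipFlop, playing a sound and rotating its yaw on a timeline.
; Peek toggles the view target between door and player inside front or back peek volumes, which activate their cameras; MoveCamera is an empty stub.
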(event OnComponentBeginOverlap(FrontOpen)
  (params (OverlappedComponent :type Primitive%20Component%20Object%20Reference) (OtherActor :type Actor%20Object%20Reference) (OtherComp :type Primitive%20Component%20Object%20Reference) (OtherBodyIndex :type Integer) (bFromSweep :type Boolean) (SweepResult :type Hit%20Result%20Structure%20%28by%20ref%29))
  (bind _door (Variables|Default|GetDoor))
  (bind _returnvalue (Transformation|GetWorldLocation _door))
  ;[1 1 1] Open/Close Door
  (bind _asfirst_person_character (Utilities|Casting|CastToFirstPersonCharacter OtherActor))
  (Variables|Default|SetCharREF _asfirst_person_character)
  (Input|EnableInput (Game|GetPlayerController 0))
  (Utilities|FlowControl|Gate true) ; enters at Open
)

(event OnComponentEndOverlap(FrontOpen)
  (params (OverlappedComponent :type Primitive%20Component%20Object%20Reference) (OtherActor :type Actor%20Object%20Reference) (OtherComp :type Primitive%20Component%20Object%20Reference) (OtherBodyIndex :type Integer))
  (bind _door (Variables|Default|GetDoor))
  (bind _returnvalue (Transformation|GetWorldLocation _door))
  ;[1 1 1] Open/Close Door
  (Utilities|Casting|CastToFirstPersonCharacter OtherActor)
  (Input|DisableInput (Game|GetPlayerController 0))
  (Utilities|FlowControl|Gate true) ; enters at Close
)

(event OnComponentBeginOverlap(FrontPeek)
  (params (OverlappedComponent :type Primitive%20Component%20Object%20Reference) (OtherActor :type Actor%20Object%20Reference) (OtherComp :type Primitive%20Component%20Object%20Reference) (OtherBodyIndex :type Integer) (bFromSweep :type Boolean) (SweepResult :type Hit%20Result%20Structure%20%28by%20ref%29))
  (Variables|Default|SetCanPeek? true)
  (Components|Activation|SetActive (Variables|Default|GetCamera1) true false))

(event OnComponentEndOverlap(FrontPeek)
  (params (OverlappedComponent :type Primitive%20Component%20Object%20Reference) (OtherActor :type Actor%20Object%20Reference) (OtherComp :type Primitive%20Component%20Object%20Reference) (OtherBodyIndex :type Integer))
  (Variables|Default|SetCanPeek? false)
  (Components|Activation|Deactivate (Variables|Default|GetCamera1)))

(event OnComponentBeginOverlap(BackPeek)
  (params (OverlappedComponent :type Primitive%20Component%20Object%20Reference) (OtherActor :type Actor%20Object%20Reference) (OtherComp :type Primitive%20Component%20Object%20Reference) (OtherBodyIndex :type Integer) (bFromSweep :type Boolean) (SweepResult :type Hit%20Result%20Structure%20%28by%20ref%29))
  (Variables|Default|SetCanPeek? true)
  (Components|Activation|SetActive (Variables|Default|GetCamera) true false))

(event OnComponentEndOverlap(BackPeek)
  (params (OverlappedComponent :type Primitive%20Component%20Object%20Reference) (OtherActor :type Actor%20Object%20Reference) (OtherComp :type Primitive%20Component%20Object%20Reference) (OtherBodyIndex :type Integer))
  (Variables|Default|SetCanPeek? false)
  (Components|Activation|Deactivate (Variables|Default|GetCamera)))

(event Custom|MoveCamera)

(event Input|ActionEvents|InputActionInteract
  (params (Key :type Key%20Structure :default "None"))
  (bind _door (Variables|Default|GetDoor))
  (bind _returnvalue (Transformation|GetWorldLocation _door))
  ;[1 1 1] Open/Close Door
  (:Pressed
    (Variables|Default|SetOpenDoor? true)
    (Utilities|FlowControl|Gate true
      (:Exit
        (if (Variables|Default|GetOpenDoor?)
          (Utilities|FlowControl|FlipFlop
            (:A
              (Audio|PlaySoundatLocation (Variables|Default|GetDoorOpen) _returnvalue "0, 0, 0" 1.0 1.0 0.0 0 0 0)
              (bind _door_2 (Timeline|DoorTimeline Play)
                (:Update
                  (Transformation|SetRelativeRotation (Variables|Default|GetDoor) (Math|Rotator|MakeRotator 0.0 0.0 (Math|Float|Lerp 0.0 1e+02 _door_2)) false false))))
            (:B
              (Audio|PlaySoundatLocation (Variables|Default|GetDoorClose) _returnvalue "0, 0, 0" 1.0 1.0 0.0 0 0 0)
              (Timeline|DoorTimeline Reverse)))
          (else
            (bind _success_ (CallFunction|ToggleCamera))
            (if _success_
              (CallFunction|MoveCamera)))))))
  (:Released
    (Variables|Default|SetOpenDoor? false)))

(event Input|ActionEvents|InputActionPeek
  (params (Key :type Key%20Structure :default "None"))
  (bind _door (Variables|Default|GetDoor))
  (bind _returnvalue (Transformation|GetWorldLocation _door))
  ;[1 1 1] Open/Close Door
  (:Pressed
    (Utilities|FlowControl|Gate true
      (:Exit
        (if (Variables|Default|GetOpenDoor?)
          (Utilities|FlowControl|FlipFlop
            (:A
              (Audio|PlaySoundatLocation (Variables|Default|GetDoorOpen) _returnvalue "0, 0, 0" 1.0 1.0 0.0 0 0 0)
              (bind _door_2 (Timeline|DoorTimeline Play)
                (:Update
                  (Transformation|SetRelativeRotation (Variables|Default|GetDoor) (Math|Rotator|MakeRotator 0.0 0.0 (Math|Float|Lerp 0.0 1e+02 _door_2)) false false))))
            (:B
              (Audio|PlaySoundatLocation (Variables|Default|GetDoorClose) _returnvalue "0, 0, 0" 1.0 1.0 0.0 0 0 0)
              (Timeline|DoorTimeline Reverse)))
          (else
            (bind _success_ (CallFunction|ToggleCamera))
            (if _success_
              (CallFunction|MoveCamera))))))))

(fn ConstructionScript)

(fn ToggleCamera
  (bind _returnvalue (Game|GetPlayerController 0))
  (if (Variables|Default|GetCanPeek?)
    (if (Variables|Default|GetIsLooking?)
      (Variables|Default|SetIsLooking? false)
      (Game|Player|SetViewTargetwithBlend _returnvalue (Variables|Default|GetCharREF) 0.3 "VTBlend_Linear" 0.0 false)
      (else
        (Variables|Default|SetIsLooking? true)
        (Game|Player|SetViewTargetwithBlend _returnvalue self 0.3 "VTBlend_Linear" 0.0 false)))
    (return true)
    (else
      (return false))))