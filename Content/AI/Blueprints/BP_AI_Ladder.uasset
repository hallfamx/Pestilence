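; BP_AI_Ladder is a smart nav link that lets AI agents climb a ladder in either direction.
; The construction script places top and bottom arrows at configurable snap offsets.
; When an agent reaches the link, the nearer arrow becomes the entry and the farther the exit.
; It sends these, the destination, ladder rotation and a from-top flag to the agent, which handles the climb.
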(event EventSmartLinkReached
  (params (Agent :type Actor%20Object%20Reference) (Destination :type Vector%20%28by%20ref%29 :default "0, 0, 0"))
  (bind _returnvalue (Transformation|GetActorLocation Agent))
  (bind _exitloc (CallFunction|GetExitLocation _returnvalue))
  (bind _enterloc (CallFunction|GetEnterLocation _returnvalue))
  ;[1 1 1] When the AI reaches the entry point on one side of the ladder, trigger the Event for moving and animating the AI thru the ladder.
  (Class|BPIParkour|OnClimbLadder(Message) Agent _enterloc _exitloc Destination (Transformation|GetActorRotation) (> (.Z (Math|Vector|BreakVector _enterloc)) (.Z (Math|Vector|BreakVector _exitloc)))))

(fn ConstructionScript
  (Transformation|SetRelativeLocation (Variables|Default|GetTopArrow) (Variables|Default|GetTopSnapOffset) false false)
  (Transformation|SetRelativeLocation (Variables|Default|GetBottomArrow) (Variables|Default|GetBottomSnapOffset) false false))

(fn GetEnterLocation
  (params (Loc :type Vector))
  (bind _toparrow (Variables|Default|GetTopArrow))
  (bind _bottomarrow (Variables|Default|GetBottomArrow))
  (bind _returnvalue (Transformation|GetWorldLocation _bottomarrow))
  (bind _returnvalue_2 (Transformation|GetWorldLocation _toparrow))
  (return (select (> (Math|Vector|VectorLength (- Loc _returnvalue_2)) (Math|Vector|VectorLength (- Loc _returnvalue))) _returnvalue _returnvalue_2)))

(fn GetExitLocation
  (params (Loc :type Vector))
  (bind _toparrow (Variables|Default|GetTopArrow))
  (bind _bottomarrow (Variables|Default|GetBottomArrow))
  (bind _returnvalue (Transformation|GetWorldLocation _bottomarrow))
  (bind _returnvalue_2 (Transformation|GetWorldLocation _toparrow))
  (return (select (< (Math|Vector|VectorLength (- Loc _returnvalue_2)) (Math|Vector|VectorLength (- Loc _returnvalue))) _returnvalue _returnvalue_2)))