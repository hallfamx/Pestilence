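; Ranged guard NPC Blueprint that adds a few event reactions to its parent class.
; On a ranged attack, its BehaviorTriggerComponent sends an area message from the guard's location to a fixed radius, with the guard as instigator.
; On death, it replaces its actor tags with a single None entry to clear them.
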(event EventBeginPlay
  (|CallParentFunction))

(event Collision|EventActorBeginOverlap
  (params (OtherActor :type Actor%20Object%20Reference)))

(event EventTick
  (params (DeltaSeconds :type Float%20%28single-precision%29)))

(event EventOnDeath
  ;[1 1 1] Remove Tags on Death
  (Variables|Default|SetTags (Utilities|Array|MakeArray "None")))

(event EventOnRangedAttack
  (Default|SendAreaMessage (Variables|Default|GetBehaviorTriggerComponent) self (Transformation|GetActorLocation) 1e+03 "NewEnumerator0"))

(fn ConstructionScript
  (|CallParentFunction))