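; Cultist NPC Blueprint that arms itself for combat and alerts nearby NPCs.
; Behavior component state events attach the weapon to the hand socket on defend or melee attack and to the unequip socket on idle.
; Entering combat and each melee swing broadcast area messages through the behavior trigger component.
; Melee attacks also play hit or swing sounds, and death overwrites the actor's tags.
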(event OnBeginDefend(BehaviorComponent)
  (bind _returnvalue (Transformation|GetActorLocation))
  (bind _self self)
  (bind _behaviortriggercomponent (Variables|Default|GetBehaviorTriggerComponent))
  (CallFunction|EquipWeapon)
  ;[1 1 1] Send Messages to nearby NPCs
  (Default|SendAreaMessage _behaviortriggercomponent _self _returnvalue 1e+03 "NewEnumerator0")
  (Default|SendAreaMessage _behaviortriggercomponent _self _returnvalue 1e+03 "NewEnumerator5"))

(event OnBeginIdle(BehaviorComponent)
  (CallFunction|UnequipWeapon))

(event OnBeginAttackMelee(BehaviorComponent)
  (bind _returnvalue (Transformation|GetActorLocation))
  (bind _self self)
  (bind _behaviortriggercomponent (Variables|Default|GetBehaviorTriggerComponent))
  (CallFunction|EquipWeapon)
  ;[1 1 1] Send Messages to nearby NPCs
  (Default|SendAreaMessage _behaviortriggercomponent _self _returnvalue 1e+03 "NewEnumerator0")
  (Default|SendAreaMessage _behaviortriggercomponent _self _returnvalue 1e+03 "NewEnumerator5"))

(event Custom|EquipWeapon
  ;[1 1 1] Equip weapons on enter Defend state
  (Transformation|AttachComponentToComponent (Variables|Default|GetWeapon) (Variables|Character|GetMesh) "weapon_socket" "KeepRelative" "KeepRelative" "KeepRelative" true))

(event Custom|UnequipWeapon
  ;[1 1 1] Unequip weapons on enter Idle state
  (Transformation|AttachComponentToComponent (Variables|Default|GetWeapon) (Variables|Character|GetMesh) "unequip_weapon_socket" "KeepRelative" "KeepRelative" "KeepRelative" true))

(event EventBeginPlay
  (|CallParentFunction))

(event Collision|EventActorBeginOverlap
  (params (OtherActor :type Actor%20Object%20Reference)))

(event EventTick
  (params (DeltaSeconds :type Float%20%28single-precision%29)))

(event EventOnDeath
  ;[1 1 1] Remove Tags on Death
  (Variables|Default|SetTags (Utilities|Array|MakeArray "None")))

(event EventOnMeleeAttack
  (params (HitSuccess :type Boolean))
  (bind _returnvalue (Transformation|GetActorLocation))
  (Utilities|FlowControl|Sequence
    (:then_0
      (Default|SendAreaMessage (Variables|Default|GetBehaviorTriggerComponent) self (Transformation|GetActorLocation) 1e+03 "NewEnumerator0"))
    (:then_1
      (if HitSuccess
        (Audio|PlaySoundatLocation "/Game/AI/Assets/Sounds/Sword/SC_Sword_Hit.SC_Sword_Hit" _returnvalue "0, 0, 0" 1.0 1.0 0.0 0 0 0)
        (else
          (Audio|PlaySoundatLocation "/Game/AI/Assets/Sounds/Sword/SC_Sword_Swing.SC_Sword_Swing" _returnvalue "0, 0, 0" 1.0 1.0 0.0 0 0 0))))))

(fn ConstructionScript
  (|CallParentFunction))