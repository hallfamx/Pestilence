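; Companion NPC Blueprint that adds weapon handling and melee attack feedback to its parent class.
; Behavior component Defend and Idle events reattach the weapon between drawn and unequipped mesh sockets, with comments flagging that this needs replication for multiplayer.
; Each melee attack broadcasts a behavior message to the surrounding area, then plays a sword hit or swing sound depending on success.
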(event OnBeginDefend(BehaviorComponent)
  (CallFunction|EquipWeapon))

(event OnBeginIdle(BehaviorComponent)
  (CallFunction|UnequipWeapon))

(event Custom|EquipWeapon
  ;[1 1 1] Equip weapons on enter Defend state (Replicate this for multiplayer)
  (Transformation|AttachComponentToComponent (Variables|Default|GetWeapon) (Variables|Character|GetMesh) "weapon_socket" "KeepRelative" "KeepRelative" "KeepRelative" true))

(event Custom|UnequipWeapon
  ;[1 1 1] Unequip weapons on enter Idle state (Replicate this for multiplayer)
  (Transformation|AttachComponentToComponent (Variables|Default|GetWeapon) (Variables|Character|GetMesh) "unequip_weapon_socket" "KeepRelative" "KeepRelative" "KeepRelative" true))

(event EventBeginPlay
  (|CallParentFunction))

(event Collision|EventActorBeginOverlap
  (params (OtherActor :type Actor%20Object%20Reference)))

(event EventTick
  (params (DeltaSeconds :type Float%20%28single-precision%29)))

(event EventOnMeleeAttack
  (params (HitSuccess :type Boolean))
  (bind _returnvalue (Transformation|GetActorLocation))
  (Utilities|FlowControl|Sequence
    (:then_0
      (Default|SendAreaMessage (Variables|Default|GetBehaviorTriggerComponent) self (Transformation|GetActorLocation) 1e+03 "NewEnumerator0"))
    (:then_1
      (if HitSuccess
        (Audio|PlaySoundatLocation "/Game/AI/Assets/Sounds/Sword/SC_Sword_Hit.SC_Sword_Hit" _returnvalue "0, 0, 0" 1.0 1.0 0.0 0 0 0)
        (else
          (Audio|PlaySoundatLocation "/Game/AI/Assets/Sounds/Sword/SC_Sword_Swing.SC_Sword_Swing" _returnvalue "0, 0, 0" 1.0 1.0 0.0 0 0 0))))))

(fn ConstructionScript
  (|CallParentFunction))