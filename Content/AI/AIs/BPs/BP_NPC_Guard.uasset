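; Guard NPC Blueprint that arms itself for defense or melee and damages the player.
; Behavior component events move the weapon between hand and unequip sockets as defend, attack and idle states change.
; Defending and attacking broadcast area messages to nearby NPCs through the behavior trigger component.
; Successful hits subtract health from the first-person character cached on melee collision overlap, with hit or swing sounds, while death resets actor tags.
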(event OnBeginDefend(BehaviorComponent)
  (bind _returnvalue (Transformation|GetActorLocation))
  (bind _self self)
  (bind _behaviortriggercomponent (Variables|Default|GetBehaviorTriggerComponent))
  (CallFunction|EquipWeapon)
  ;[1 1 1] Send Messages to nearby NPCs
  (Default|SendAreaMessage _behaviortriggercomponent _self _returnvalue 1e+03 "NewEnumerator0")
  (Default|SendAreaMessage _behaviortriggercomponent _self _returnvalue 1e+03 "NewEnumerator5"))

(event OnBeginIdle(BehaviorComponent)
  (CallFunction|UnequipWeapon))

(event OnBeginAttackMelee(BehaviorComponent)
  (bind _returnvalue (Transformation|GetActorLocation))
  (bind _self self)
  (bind _behaviortriggercomponent (Variables|Default|GetBehaviorTriggerComponent))
  (CallFunction|EquipWeapon)
  ;[1 1 1] Send Messages to nearby NPCs
  (Default|SendAreaMessage _behaviortriggercomponent _self _returnvalue 1e+03 "NewEnumerator0")
  (Default|SendAreaMessage _behaviortriggercomponent _self _returnvalue 1e+03 "NewEnumerator5"))

(event OnEndAttackMelee(BehaviorComponent)
  (CallFunction|UnequipWeapon))

(event OnComponentBeginOverlap(MeleeCollision)
  (params (OverlappedComponent :type Primitive%20Component%20Object%20Reference) (OtherActor :type Actor%20Object%20Reference) (OtherComp :type Primitive%20Component%20Object%20Reference) (OtherBodyIndex :type Integer) (bFromSweep :type Boolean) (SweepResult :type Hit%20Result%20Structure%20%28by%20ref%29))
  (bind _asfirst_person_character (Utilities|Casting|CastToFirstPersonCharacter OtherActor)))

(event Custom|UnequipGun
  (Transformation|AttachComponentToComponent (Variables|Default|GetWeapon) (Variables|Character|GetMesh) "unequip_weapon_socket" "KeepRelative" "KeepRelative" "KeepRelative" true))

(event Custom|EquipWeapon
  ;[1 1 1] Equip weapons
  (Transformation|AttachComponentToComponent (Variables|Default|GetWeapon) (Variables|Character|GetMesh) "weapon_socket" "KeepRelative" "KeepRelative" "KeepRelative" true))

(event Custom|EquipGun
  (Transformation|AttachComponentToComponent (Variables|Default|GetWeapon) (Variables|Character|GetMesh) "weapon_socket" "KeepRelative" "KeepRelative" "KeepRelative" true))

(event Custom|UnequipWeapon
  ;[1 1 1] Unequip Weapons
  (Transformation|AttachComponentToComponent (Variables|Default|GetWeapon) (Variables|Character|GetMesh) "unequip_weapon_socket" "KeepRelative" "KeepRelative" "KeepRelative" true))

(event EventBeginPlay
  (|CallParentFunction))

(event EventOnDeath
  ;[1 1 1] Remove Tags on Death
  (Variables|Default|SetTags (Utilities|Array|MakeArray "None")))

(event EventOnMeleeAttack
  (params (HitSuccess :type Boolean))
  (bind _returnvalue (Transformation|GetActorLocation))
  (Utilities|FlowControl|Sequence
    (:then_0
      (Default|SendAreaMessage (Variables|Default|GetBehaviorTriggerComponent) self (Transformation|GetActorLocation) 1e+03 "NewEnumerator0"))
    (:then_1
      (if HitSuccess
        (Audio|PlaySoundatLocation "/Game/AI/Assets/Sounds/Sword/SC_Sword_Hit.SC_Sword_Hit" _returnvalue "0, 0, 0" 1.0 1.0 0.0 0 0 0)
        (Variables|/Game/FirstPersonBP/Blueprints/FirstPersonCharacter.FirstPersonCharacter_C|SetHealth (stale OnComponentBeginOverlap(MeleeCollision) _asfirst_person_character) (- (Variables|/Game/FirstPersonBP/Blueprints/FirstPersonCharacter.FirstPersonCharacter_C|GetHealth (stale OnComponentBeginOverlap(MeleeCollision) _asfirst_person_character)) 4))
        (else
          (Audio|PlaySoundatLocation "/Game/AI/Assets/Sounds/Sword/SC_Sword_Swing.SC_Sword_Swing" _returnvalue "0, 0, 0" 1.0 1.0 0.0 0 0 0))))))

(fn ConstructionScript
  (|CallParentFunction))