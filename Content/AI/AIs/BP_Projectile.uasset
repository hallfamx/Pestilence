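; Projectile actor that deals damage on sphere overlap and then destroys itself, crediting its owner as damage causer.
; NPCs take a hardcoded damage amount only when their capsule is hit while alive; otherwise the projectile passes through that overlap without effect.
; Any other overlapped actor takes the Damage variable's amount.
; A blocking hit on the sphere destroys the projectile without applying damage.
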(event OnComponentHit(Sphere)
  (params (HitComponent :type Primitive%20Component%20Object%20Reference) (OtherActor :type Actor%20Object%20Reference) (OtherComp :type Primitive%20Component%20Object%20Reference) (NormalImpulse :type Vector :default "0, 0, 0") (Hit :type Hit%20Result%20Structure%20%28by%20ref%29))
  (Actor|DestroyActor))

(event OnComponentBeginOverlap(Sphere)
  (params (OverlappedComponent :type Primitive%20Component%20Object%20Reference) (OtherActor :type Actor%20Object%20Reference) (OtherComp :type Primitive%20Component%20Object%20Reference) (OtherBodyIndex :type Integer) (bFromSweep :type Boolean) (SweepResult :type Hit%20Result%20Structure%20%28by%20ref%29))
  (bind _asbp_npc_base (Utilities|Casting|CastToBP_NPC_Base OtherActor)
    (:then
      (if (== OtherComp (Variables|/Script/Engine.Character|GetCapsuleComponent _asbp_npc_base))
        (if (Variables|/Game/AI/Blueprints/BP_BehaviorComponent.BP_BehaviorComponent_C|GetIsAlive (Variables|/Game/AI/Blueprints/BP_NPC_Base.BP_NPC_Base_C|GetBehaviorComponent _asbp_npc_base))
          (Game|Damage|ApplyDamage _asbp_npc_base 5.0 0 (Components|GetOwner))
          (Actor|DestroyActor :!label _label))))
    (:CastFailed
      (Game|Damage|ApplyDamage OtherActor (Variables|Default|GetDamage) 0 (Components|GetOwner))
      (goto _label))))

(fn ConstructionScript)