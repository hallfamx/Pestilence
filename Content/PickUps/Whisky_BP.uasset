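; Whisky pickup actor that the first-person character can collect or that can shatter and make noise.
; A Box overlap enables input and opens a gate, so Interact sets HasWhisky on the character, plays a pickup sound and destroys the actor.
; Fracturing the destructible mesh plays a break sound, reports a "Glass" AI noise event, removes the Box to block pickup and destroys the debris after a delay.
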(event OnComponentBeginOverlap(Box)
  (params (OverlappedComponent :type Primitive%20Component%20Object%20Reference) (OtherActor :type Actor%20Object%20Reference) (OtherComp :type Primitive%20Component%20Object%20Reference) (OtherBodyIndex :type Integer) (bFromSweep :type Boolean) (SweepResult :type Hit%20Result%20Structure%20%28by%20ref%29))
  (bind _asfirst_person_character (Utilities|Casting|CastToFirstPersonCharacter OtherActor))
  (Variables|Default|SetCharREF _asfirst_person_character)
  (Input|EnableInput (Game|GetPlayerController 0))
  (Utilities|FlowControl|Gate true) ; enters at Open
)

(event OnComponentEndOverlap(Box)
  (params (OverlappedComponent :type Primitive%20Component%20Object%20Reference) (OtherActor :type Actor%20Object%20Reference) (OtherComp :type Primitive%20Component%20Object%20Reference) (OtherBodyIndex :type Integer))
  (Utilities|Casting|CastToFirstPersonCharacter OtherActor)
  (Input|DisableInput (Game|GetPlayerController 0))
  (Utilities|FlowControl|Gate true) ; enters at Close
)

(event OnComponentFracture(whisky_DM)
  (params (HitPoint :type Vector%20%28by%20ref%29 :default "0, 0, 0") (HitDirection :type Vector%20%28by%20ref%29 :default "0, 0, 0"))
  (bind _returnvalue (Transformation|GetActorLocation))
  (Audio|PlaySoundatLocation (Variables|Default|GetBreakSound) _returnvalue "0, 0, 0" 1.0 1.0 0.0 0 0 0)
  (Class|AISenseHearing|ReportNoiseEvent _returnvalue 2.0 0 5e+02 "Glass")
  (Components|DestroyComponent (Variables|Default|GetBox))
  (Utilities|FlowControl|Delay 35.0)
  (Actor|DestroyActor))

(event Input|ActionEvents|InputActionInteract
  (params (Key :type Key%20Structure :default "None"))
  (:Pressed
    (Utilities|FlowControl|Gate true
      (:Exit
        (Variables|/Game/FirstPersonBP/Blueprints/FirstPersonCharacter.FirstPersonCharacter_C|SetHasWhisky (Variables|Default|GetCharREF) true)
        (Audio|PlaySoundatLocation (Variables|Default|GetPickUpSound) (Transformation|GetActorLocation) "0, 0, 0" 1.0 1.0 0.0 0 0 0)
        (Utilities|FlowControl|Delay 0.01)
        (Actor|DestroyActor)))))

(fn ConstructionScript)