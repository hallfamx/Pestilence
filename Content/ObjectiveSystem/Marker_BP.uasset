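; Marker actor that shows the player's distance to it, likely as an objective marker given its ObjectiveSystem folder.
; Every tick it measures the distance from itself to the first player character, converts it to whole meters and appends an "m" suffix.
; The text is pushed to the user widget of its WidgetMarker component through UpdateTextMessage.
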(event EventTick
  (params (DeltaSeconds :type Float%20%28single-precision%29))
  (Class|MarkerBPI|UpdateText(Message) (UserInterface|GetUserWidgetObject (Variables|Default|GetWidget_Marker)) (Utilities|Text|ToText(String) (Utilities|String|Append (Utilities|String|ToString(Integer) (Math|Float|Truncate (/ (Math|Vector|Distance(Vector) (Transformation|GetActorLocation) (Transformation|GetActorLocation (Game|GetPlayerCharacter 0))) 1e+02))) "m"))))

(fn ConstructionScript)