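; ObjectiveEnd_BP is a trigger actor that completes a main or side objective when the first-person character enters its box.
; On overlap it checks the MainQuest flag and compares its Objective to the character's matching current objective.
; On a match it clears that objective, calls the matching slide-off function on the character, plays a completion sound and destroys itself.
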(event OnComponentBeginOverlap(Box)
  (params (OverlappedComponent :type Primitive%20Component%20Object%20Reference) (OtherActor :type Actor%20Object%20Reference) (OtherComp :type Primitive%20Component%20Object%20Reference) (OtherBodyIndex :type Integer) (bFromSweep :type Boolean) (SweepResult :type Hit%20Result%20Structure%20%28by%20ref%29))
  (bind _asfirst_person_character (Utilities|Casting|CastToFirstPersonCharacter OtherActor))
  (if (Variables|Default|GetMainQuest)
    (if (Utilities|Enum|Equal(Enum) (Variables|/Game/FirstPersonBP/Blueprints/FirstPersonCharacter.FirstPersonCharacter_C|GetCurrentObjective _asfirst_person_character) (Variables|Default|GetObjective))
      (Variables|/Game/FirstPersonBP/Blueprints/FirstPersonCharacter.FirstPersonCharacter_C|SetCurrentObjective _asfirst_person_character "")
      ;[1 1 1] Obj done
      (Default|SlideOff _asfirst_person_character)
      (Audio|PlaySound2D (Variables|Default|GetObjectiveCompleteSound) 1.0 1.0 0.0 0 0 :!label _label)
      (Actor|DestroyActor))
    (elif (Utilities|Enum|Equal(Enum) (Variables|/Game/FirstPersonBP/Blueprints/FirstPersonCharacter.FirstPersonCharacter_C|GetCurrentObjective_Side _asfirst_person_character) (Variables|Default|GetObjective))
      (Variables|/Game/FirstPersonBP/Blueprints/FirstPersonCharacter.FirstPersonCharacter_C|SetCurrentObjective_Side _asfirst_person_character "")
      (Default|SlideOffSide _asfirst_person_character)
      (goto _label))))

(fn ConstructionScript)